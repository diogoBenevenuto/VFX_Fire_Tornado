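; Area-of-effect VFX actor that plays a configurable Niagara system and destroys itself after a set delay.
; The construction script assigns the system and passes Scale as vector and float, plus ImpactDelay and optional color overrides only when ImpactDelay is positive.
; BeginPlay reassigns the system with override parameters reset, offsets the actor by Location, sets its Rotation, then starts the destroy timer.
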(event `self.ReceiveBeginPlay`
  (`self.SpawnAoE`)
  (`KismetSystemLibrary.Delay` (`self.DelayBeforeDestroying`))
  (`self.K2_DestroyActor`))

(event `SpawnAoE`
  (`NiagaraComponent.SetAsset` (`self.AreaOfEffectNiagara`) (`self.VFXAreaOfEffectNiagara`) true)
  (`self.K2_SetActorLocationAndRotation` (+ (`self.K2_GetActorLocation`) (`self.Location`)) (`self.Rotation`)))

(fn `UserConstructionScript`
  (bind _scale (`self.Scale`))
  (bind _impactdelay (`self.ImpactDelay`))
  (bind _areaofeffectniagara (`self.AreaOfEffectNiagara`))
  (if (`KismetSystemLibrary.IsValid` (`self.VFXAreaOfEffectNiagara`))
    (`NiagaraComponent.SetAsset` _areaofeffectniagara (`self.VFXAreaOfEffectNiagara`) true)
    (`NiagaraComponent.SetVariableVec3` _areaofeffectniagara "Scale" _scale)
    (`NiagaraComponent.SetVariableFloat` _areaofeffectniagara "Scale" (.x _scale))
    (if (> _impactdelay 0.0)
      (`NiagaraComponent.SetVariableFloat` _areaofeffectniagara "ImpactDelay" _impactdelay)
      (if (`self.ChangeColor01`)
        (`NiagaraComponent.SetVariableLinearColor` (`self.AreaOfEffectNiagara`) "Color01" (`self.Color01`)))
      (if (`self.ChangeColor02`)
        (`NiagaraComponent.SetVariableLinearColor` (`self.AreaOfEffectNiagara`) "Color02" (`self.Color02`))))))